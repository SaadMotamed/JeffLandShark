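; Lobby player controller that shows the lobby UI and reports the player's info and ready status to the lobby game mode.
; On begin play, local controllers create the lobby widget with cursor and game-and-UI input, then registration with Lobby_GM follows where the cast succeeds.
; A delayed retry event resends info, and a ready toggle pushes the flipped status to Lobby_GM.
; Match start shows a loading screen and disables input.
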(event Custom|OnStartMatch
  (Default|ShowLoadingScreen (Variables|Default|GetLobbyUIRef))
  (Input|DisableInput self))

(event Custom|TryAgainUpdatingLobbyInfo
  (Utilities|FlowControl|Delay 0.1)
  (bind _aslobby_gm (Utilities|Casting|CastToLobby_GM (Game|GetGameMode)))
  (Default|UpdatePlayerLobbyInfo _aslobby_gm self))

(event Custom|ToggleReadyStatusOnServer
  (bind _playerlobbyinfopc (Variables|Default|GetPlayerLobbyInfoPC))
  (Utilities|Struct|SetmembersinS_PlayerLobbyInfo _playerlobbyinfopc (not (.Ready (Utilities|Struct|BreakS_PlayerLobbyInfo _playerlobbyinfopc))))
  (bind _aslobby_gm (Utilities|Casting|CastToLobby_GM (Game|GetGameMode)))
  (Default|UpdatePlayerLobbyInfo _aslobby_gm self))

(event EventBeginPlay
  (CallFunction|SetUp)
  (bind _aslobby_gm (Utilities|Casting|CastToLobby_GM (Game|GetGameMode)))
  (Default|UpdatePlayerLobbyInfo _aslobby_gm self))

(fn ConstructionScript)

(fn SetUp
  (if (Pawn|IsLocalPlayerController)
    (Variables|Default|SetbShowMouseCursor true)
    (Input|SetInputModeGameandUI self 0 "DoNotLock" false false)
    (bind _returnvalue (UserInterface|CreateWidget "/Game/Dev/Blueprints/Lobby/WB_LobbyUI.WB_LobbyUI_C"))
    (bind _output_get (Variables|Default|SetLobbyUIRef _returnvalue))
    (UserInterface|Viewport|AddtoViewport _output_get 0)))